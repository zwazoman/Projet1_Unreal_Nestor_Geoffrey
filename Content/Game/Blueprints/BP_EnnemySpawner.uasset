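; Zombie wave spawner that starts shortly after play, spawning BP_Zombie at random spawn points and showing each wave number on the player HUD.
; A looping timer spawns the wave's quota, and the next wave starts when ZombieDied counts the living down to zero.
; Each wave grows and spawns faster, with every tenth setting a never-cleared mega-wave flag that doubles count and shortens the interval.
; Group-spawn logic is unfinished and disconnected.
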(event Custom|Spawn%20Enemy
  ;[1 1 1] Spawning zombies for waves
  (if (> (Variables|Default|GetZombies%20to%20Spawn) 0)
    (Math|Integer|DecrementInt (Variables|Default|GetZombies%20to%20Spawn)
      (:%20%20
        (bind _returnvalue (Game|SpawnActorfromClass "/Game/Game/Blueprints/BP_Zombie.BP_Zombie_C" (Math|Conversions|ToTransform(Vector) (Transformation|GetActorLocation (.OutItem (Utilities|Array|Random (Variables|Default|GetSpawnPoints))))) "AlwaysSpawn" "MultiplyWithRoot" 0 0))
        (Variables|/Game/Game/Blueprints/BP_Zombie.BP_Zombie_C|SetSpawner _returnvalue self)))))

(event Custom|Spawn%20New%20Wave
  ;[1 1 1] Spawning zombies for waves
  (Utilities|Time|SetTimerbyEvent (delegate Custom|Spawn%20Enemy) (Variables|Default|GetCurrent%20Spawn%20Rate) true))

(event Custom|Next%20Wave
  ;[1 1 1] Wave Handling
  (if (!= (Math|Integer|%(Integer) (Variables|Default|GetCurrent%20Wave) 10) 0)
    _
    (else
      (Variables|Default|SetIsMegaWave true)))
  (CallFunction|SpawnWaveUI)
  (Math|Integer|IncrementInt (Variables|Default|GetCurrent%20Wave)
    (:%20%20
      (bind _output_get (Variables|Default|SetZombies%20Total%20Spawn%20Count (Math|Float|Round (* (Math|Conversions|ToFloat(Integer) (Variables|Default|GetZombies%20Total%20Spawn%20Count)) 1.3))))
      (bind _output_get_2 (Variables|Default|SetZombies%20to%20Spawn _output_get))
      (Variables|Default|SetCurrent%20Zombie%20Count _output_get_2)
      (bind _output_get_3 (Variables|Default|SetSpawnRate (* (Variables|Default|GetSpawnRate) 0.9)))
      (Variables|Default|SetCurrent%20Spawn%20Rate _output_get_3)
      ;[1 1 1] Mega Wave Handle
      (if (Variables|Default|GetIsMegaWave)
        (bind _output_get_4 (Variables|Default|SetZombies%20to%20Spawn (* (Variables|Default|GetZombies%20to%20Spawn) 2)))
        (Variables|Default|SetCurrent%20Zombie%20Count _output_get_4)
        (Variables|Default|SetCurrent%20Spawn%20Rate (* (Variables|Default|GetCurrent%20Spawn%20Rate) 0.3)))
      (CallFunction|SpawnNewWave))))

(event Custom|Zombie%20Died
  ;[1 1 1] Wave End Handling
  (bind _result (Math|Integer|DecrementInt (Variables|Default|GetCurrent%20Zombie%20Count))
    (:%20%20
      (if (<= _result 0)
        (CallFunction|NextWave)))))

(event Custom|Spawn%20Wave%20UI
  ;[1 1 1] UI
  (bind _asbp_player (Utilities|Casting|CastToBP_PLAYER (Game|GetPlayerCharacter 0)))
  (Default|ShowWaveNumber (Variables|/Game/Game/Blueprints/BP_PLAYER.BP_PLAYER_C|GetHUD _asbp_player) (Variables|Default|GetCurrent%20Wave))
  (Utilities|FlowControl|Delay 2.0)
  (Default|HideWaveNulber (Variables|/Game/Game/Blueprints/BP_PLAYER.BP_PLAYER_C|GetHUD _asbp_player)))

(event EventBeginPlay
  (Utilities|FlowControl|Delay 0.2)
  (CallFunction|NextWave))

(fn ConstructionScript)